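; Actor that appears as either a Man or a Knight, following the LightDark flag on the LightAndDark game mode.
; Visibility refreshes on BeginPlay, on SwapCharacter input, and when Tick sees the Reset flag; the flag itself is only read here.
; Pressing Interact while overlapping a Death actor destroys this actor if LightDark is true, the state that shows the Man.
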(event EventBeginPlay
  (Input|EnableInput (Game|GetPlayerController 0))
  (bind _aslight_and_dark (Utilities|Casting|CastToLightAndDark (Game|GetGameMode))
    (:then
      _)
    (:CastFailed
      (Development|PrintString "Cast to 'LightAndDark' Failed")))
  (Rendering|SetVisibility (Variables|Default|GetKnight) (not (Variables|/Game/LightAndDark.LightAndDark_C|GetlightDark _aslight_and_dark)) true)
  (Rendering|SetVisibility (Variables|Default|GetMan) (Variables|/Game/LightAndDark.LightAndDark_C|GetlightDark _aslight_and_dark) true))

(event EventTick
  (params (DeltaSeconds :type Float%20%28single-precision%29))
  (if (Variables|Default|Getreset)
    (Variables|Default|Setreset false)
    (bind _aslight_and_dark (Utilities|Casting|CastToLightAndDark (Game|GetGameMode))
      (:then
        _)
      (:CastFailed
        (Development|PrintString "Cast to 'LightAndDark' Failed")))
    (Rendering|SetVisibility (Variables|Default|GetKnight) (not (Variables|/Game/LightAndDark.LightAndDark_C|GetlightDark _aslight_and_dark)) true)
    (Rendering|SetVisibility (Variables|Default|GetMan) (Variables|/Game/LightAndDark.LightAndDark_C|GetlightDark _aslight_and_dark) true)))

(event Collision|EventActorBeginOverlap
  (params (OtherActor :type Actor%20Object%20Reference))
  (bind _asdeath (Utilities|Casting|CastToDeath OtherActor)))

(event Input|ActionEvents|InputActionSwapCharacter
  (params (Key :type Key%20Structure :default "None"))
  (:Pressed
    (bind _aslight_and_dark (Utilities|Casting|CastToLightAndDark (Game|GetGameMode))
      (:then
        _)
      (:CastFailed
        (Development|PrintString "Cast to 'LightAndDark' Failed")))
    (Rendering|SetVisibility (Variables|Default|GetKnight) (not (Variables|/Game/LightAndDark.LightAndDark_C|GetlightDark _aslight_and_dark)) true)
    (Rendering|SetVisibility (Variables|Default|GetMan) (Variables|/Game/LightAndDark.LightAndDark_C|GetlightDark _aslight_and_dark) true)))

(event Input|ActionEvents|InputActionInteract
  (params (Key :type Key%20Structure :default "None"))
  (:Pressed
    (if (Collision|IsOverlappingActor (stale Collision|EventActorBeginOverlap _asdeath) :!class /Script/Engine.Actor)
      (if (Variables|/Game/LightAndDark.LightAndDark_C|GetlightDark (stale EventBeginPlay _aslight_and_dark))
        (Actor|DestroyActor)))))

(fn ConstructionScript)